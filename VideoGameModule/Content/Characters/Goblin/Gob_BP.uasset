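; Goblin enemy character that chases the player, attacks in melee and can trigger game over.
; Tick handles ragdoll death at zero health, moves toward the player within range or back to a hardcoded start point, and toggles the AnimBP attack flag by distance.
; Attack-collision overlap during attacks damages Char_BP, pausing with GameOverHUD when its health runs out.
; BeginPlay also creates the main HUD.
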(event OnComponentBeginOverlap(GobAttackCollision)
  (params (OverlappedComponent :type Primitive%20Component%20Object%20Reference) (OtherActor :type Actor%20Object%20Reference) (OtherComp :type Primitive%20Component%20Object%20Reference) (OtherBodyIndex :type Integer) (bFromSweep :type Boolean) (SweepResult :type Hit%20Result%20Structure%20%28by%20ref%29))
  (bind _returnvalue (Game|GetPlayerController 0))
  (bind _aschar_bp (Utilities|Casting|CastToChar_BP OtherActor))
  (if (== (Variables|/Script/Engine.Character|GetCapsuleComponent _aschar_bp) OtherComp)
    (bind _asgob_anim_bp (Utilities|Casting|CastToGob_AnimBP (Components|SkeletalMesh|GetAnimInstance (Variables|Character|GetMesh))))
    (if (Variables|/Game/Characters/Goblin/Gob_AnimBP.Gob_AnimBP_C|GetIsAttack _asgob_anim_bp)
      (Variables|/Game/Characters/PlayerCharacter/Char_BP.Char_BP_C|SetCharHealth _aschar_bp (- (Variables|/Game/Characters/PlayerCharacter/Char_BP.Char_BP_C|GetCharHealth _aschar_bp) 0.1))
      (if (<= (Variables|/Game/Characters/PlayerCharacter/Char_BP.Char_BP_C|GetCharHealth _aschar_bp) 0.0)
        (bind _returnvalue_2 (UserInterface|CreateWidget "/Game/Widgets/Game_Over/GameOverHUD.GameOverHUD_C"))
        (UserInterface|Viewport|AddtoViewport _returnvalue_2 0)
        (Game|SetGamePaused true)
        (Variables|/Script/Engine.PlayerController|SetbShowMouseCursor _returnvalue true)
        (Input|SetInputModeUIOnly _returnvalue 0 "DoNotLock")))))

(event EventBeginPlay
  (bind _returnvalue (UserInterface|CreateWidget "/Game/Widgets/HUD/MainHUD.MainHUD_C"))
  (UserInterface|Viewport|AddtoViewport _returnvalue 0)
  (Variables|Default|SetGobStart "3193.000000,-149.000000,182.956436"))

(event EventTick
  (params (DeltaSeconds :type Float%20%28single-precision%29))
  (Utilities|FlowControl|Sequence
    (:then_0
      (if (<= (Variables|Default|GetGobHealth) 0.0)
        (if (not (Variables|Default|GetGobDead))
          (Variables|Default|SetGobDead true)
          (Physics|SetSimulatePhysics (Variables|Character|GetMesh) true)
          (Components|DestroyComponent (Variables|Default|GetGobAttackCollision)))))
    (:then_1
      (Utilities|Time|SetTimerbyFunctionName 0 "" 1.0 true)
      (Utilities|FlowControl|Sequence
        (:then_1
          (if (< (Math|Vector|Distance(Vector) (Transformation|GetActorLocation (Game|GetPlayerCharacter 0)) (Transformation|GetActorLocation)) 1e+03)
            (AI|Navigation|SimpleMovetoActor (Pawn|GetController) (Game|GetPlayerCharacter 0))
            (else
              (AI|Navigation|MovetoLocation (AI|GetAIController (Components|GetOwner)) (Variables|Default|GetGobStart) 5e+01 true true true true 0))))
        (:then_2
          (if (< (Math|Vector|Distance(Vector) (Transformation|GetActorLocation (Game|GetPlayerCharacter 0)) (Transformation|GetActorLocation)) 175.0)
            (bind _asgob_anim_bp (Utilities|Casting|CastToGob_AnimBP (Components|SkeletalMesh|GetAnimInstance (Variables|Character|GetMesh))))
            (Variables|/Game/Characters/Goblin/Gob_AnimBP.Gob_AnimBP_C|SetIsAttack _asgob_anim_bp true)
            (else
              (bind _asgob_anim_bp_2 (Utilities|Casting|CastToGob_AnimBP (Components|SkeletalMesh|GetAnimInstance (Variables|Character|GetMesh))))
              (Variables|/Game/Characters/Goblin/Gob_AnimBP.Gob_AnimBP_C|SetIsAttack _asgob_anim_bp_2 false))))))))

(fn ConstructionScript)